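; Enemy bot character that chases the player's MainCharacter on sight and deals melee damage, reduced when the player blocks.
; PawnSensing drives AIMoveTo, with a 1.5-second hit cooldown, state-gated looping animations and a retriggerable delay that clears sight.
; Tick updates a player-facing health bar, spins the bot around when hit unseen, and destroys it at zero HP, notifying WaveManager.
; DifChange defines health, damage and speed for three difficulty levels.
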(event OnSeePawn(PawnSensing)
  (params (Pawn :type Pawn%20Object%20Reference))
  ;[1 1 1] Bot movement logic
  (bind _asmain_character (Utilities|Casting|CastToMainCharacter Pawn))
  (Variables|Default|SetSeePlayer? true)
  (Utilities|FlowControl|Sequence
    (:then_0
      (if (not (Variables|Default|GetCollided?))
        (if (!= (Variables|Default|GetState) 1)
          (Components|Animation|PlayAnimation (Variables|Character|GetMesh) "/Game/Units/bot/bot_lowpoly2_армаша_run_for_bot.bot_lowpoly2_армаша_run_for_bot" true))
        (Variables|Default|SetState 1)
        (AI|AIMoveTo self "0, 0, 0" _asmain_character 5.0 false
          (:OnSuccess
            ;[1 1 1] Attack Logic
            (if (not (Variables|Default|GetCollided?))
              (Variables|Default|SetState 2)
              (bind _asmain_character_2 (Utilities|Casting|CastToMainCharacter _asmain_character))
              (if (Variables|/Game/Blueprints/MainCharacter.MainCharacter_C|Getblocking? _asmain_character_2)
                (Variables|/Game/Blueprints/MainCharacter.MainCharacter_C|Sethp _asmain_character_2 (- (Variables|/Game/Blueprints/MainCharacter.MainCharacter_C|Gethp _asmain_character_2) (Variables|Default|GetDam_with_block)))
                (else
                  (Variables|/Game/Blueprints/MainCharacter.MainCharacter_C|Sethp _asmain_character_2 (- (Variables|/Game/Blueprints/MainCharacter.MainCharacter_C|Gethp _asmain_character_2) (Variables|Default|GetDamage)))))
              (Variables|Default|SetCollided? true)
              (Utilities|FlowControl|Delay 1.5)
              (Variables|Default|SetCollided? false))))
        (else
          (Components|Movement|StopMovementImmediately (Variables|Character|GetCharacterMovement))
          (if (!= (Variables|Default|GetState) 3)
            (Components|Animation|PlayAnimation (Variables|Character|GetMesh) "/Game/Units/bot/bot_lowpoly3_армаша_bot_hitting_actor.bot_lowpoly3_армаша_bot_hitting_actor" true))
          (Variables|Default|SetState 3))))
    (:then_1
      (Utilities|FlowControl|RetriggerableDelay 0.2)
      (Variables|Default|SetSeePlayer? false))))

(event OnComponentBeginOverlap(Box)
  (params (OverlappedComponent :type Primitive%20Component%20Object%20Reference) (OtherActor :type Actor%20Object%20Reference) (OtherComp :type Primitive%20Component%20Object%20Reference) (OtherBodyIndex :type Integer) (bFromSweep :type Boolean) (SweepResult :type Hit%20Result%20Structure%20%28by%20ref%29))
  ;[1 1 1] Attack logic
)

(event EventTick
  (params (DeltaSeconds :type Float%20%28single-precision%29))
  (Utilities|FlowControl|Sequence
    (:then_0
      (Utilities|HpBarSys))
    (:then_1
      (Utilities|LogicOfBackstabbyPlayer))
    (:then_2
      (Utilities|DyingLogic))
    (:then_3
      (if (not (Variables|Default|GetSeePlayer?))
        (if (!= (Variables|Default|GetState) 0)
          (Components|Animation|PlayAnimation (Variables|Character|GetMesh) "/Game/Units/bot/bot_lowpoly2_армаша_searching_002.bot_lowpoly2_армаша_searching_002" true)
          (Components|Movement|StopMovementImmediately (Variables|Character|GetCharacterMovement)))
        (Variables|Default|SetState 0)))))

(fn ConstructionScript)

(fn StateChange
  (if (> (Math|Vector|VectorLength (Variables|/Script/Engine.MovementComponent|GetVelocity (Variables|Character|GetCharacterMovement))) 0.0)
    (if (not false)
      (Variables|Default|SetState 1)
      (else
        (Variables|Default|SetState 2)))
    (else
      (Variables|Default|SetState 0))))

(fn DifChange
  (if (== (Variables|Default|GetDifLevel) 2)
    (Variables|Default|Sethp 1e+02)
    (Variables|Default|Sethp_Max 1e+02)
    (Variables|Default|SetDamage 0.2)
    (Variables|/Script/Engine.CharacterMovementComponent|SetMaxWalkSpeed (Variables|Character|GetCharacterMovement) 7e+02)
    (Variables|Default|SetDam_with_block 0.05)
    (elif (== (Variables|Default|GetDifLevel) 1)
      (Variables|Default|Sethp 5e+01)
      (Variables|Default|Sethp_Max 5e+01)
      (Variables|Default|SetDamage 0.1)
      (Variables|/Script/Engine.CharacterMovementComponent|SetMaxWalkSpeed (Variables|Character|GetCharacterMovement) 5.5e+02)
      (Variables|Default|SetDam_with_block 0.0)
      (elif (== (Variables|Default|GetDifLevel) 3)
        (Variables|Default|Sethp 1.5e+02)
        (Variables|Default|Sethp_Max 1.5e+02)
        (Variables|Default|SetDamage 0.34)
        (Variables|/Script/Engine.CharacterMovementComponent|SetMaxWalkSpeed (Variables|Character|GetCharacterMovement) 8e+02)
        (Variables|Default|SetDam_with_block 0.2)))))