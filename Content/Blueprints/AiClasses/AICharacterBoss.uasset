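; AI boss character that scales its combat stats by difficulty and reports its death to a boss counter.
; DifChange maps three DifLevel values to health, damage, blocked damage and walk speed, with level 2 having the lowest health and damage but the fastest speed.
; DyingLogic destroys the actor at zero health, then calls MinusBoss on each element of an array and prints its remaining Bosses count.
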(event EventTick
  (params (DeltaSeconds :type Float%20%28single-precision%29))
  (|CallParentFunction DeltaSeconds) ; This node is disabled and will not be called.\nDrag off pins to build functionality.
)

(fn ConstructionScript
  (|CallParentFunction))

(fn DifChange
  (if (== (Variables|Default|GetDifLevel) 2)
    (Variables|Default|Sethp 1e+02)
    (Variables|Default|Sethp_Max 1e+02)
    (Variables|Default|SetDamage 0.2)
    (Variables|/Script/Engine.CharacterMovementComponent|SetMaxWalkSpeed (Variables|Character|GetCharacterMovement) 7e+02)
    (Variables|Default|SetDam_with_block 0.05)
    (elif (== (Variables|Default|GetDifLevel) 1)
      (Variables|Default|Sethp 2e+02)
      (Variables|Default|Sethp_Max 2e+02)
      (Variables|Default|SetDamage 0.5)
      (Variables|/Script/Engine.CharacterMovementComponent|SetMaxWalkSpeed (Variables|Character|GetCharacterMovement) 5.5e+02)
      (Variables|Default|SetDam_with_block 0.1)
      (elif (== (Variables|Default|GetDifLevel) 3)
        (Variables|Default|Sethp 3e+02)
        (Variables|Default|Sethp_Max 3e+02)
        (Variables|Default|SetDamage 1.0)
        (Variables|/Script/Engine.CharacterMovementComponent|SetMaxWalkSpeed (Variables|Character|GetCharacterMovement) 6.5e+02)
        (Variables|Default|SetDam_with_block 0.34)))))

(fn DyingLogic
  (if (<= (Variables|Default|Gethp) 0.0)
    (Actor|DestroyActor)
    (for _array_element 0
      (Default|MinusBoss _array_element)
      (Development|PrintString (Utilities|String|ToString(Integer) (Variables|/Game/Blueprints/WaveManager.WaveManager_C|GetBosses _array_element))))))